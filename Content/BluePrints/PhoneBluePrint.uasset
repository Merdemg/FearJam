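; A phone actor that plays a voice message in the world when interacted with.
; Interact prints a debug string and calls PlayVoiceOver, which plays the VoiceOver sound at the actor's location.
; It supplies the prompt "Listen to Voice Message", but IsInteractable always returns false and WriteToNotebook returns an empty string.
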(event EventBeginPlay)

(event Collision|EventActorBeginOverlap
  (params (OtherActor :type Actor%20Object%20Reference)))

(event EventTick
  (params (DeltaSeconds :type Float%20%28single-precision%29)))

(event EventPlayVoiceOver
  (Audio|PlaySoundatLocation (Variables|Default|Getvoice%20over) (Transformation|GetActorLocation) "0, 0, 0" 1.0 1.0 0.0 0 0 0))

(event EventInteract
  (Development|PrintString "INTERACT!!!")
  (CallFunction|PlayVoiceOver))

(fn ConstructionScript)

(fn GetString
  (return "Listen to Voice Message"))

(fn IsInteractable
  (return false))

(fn WritetoNotebook
  (return ""))