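; Notebook pickup actor that gives the player the notebook as a tutorial step.
; After a short BeginPlay delay it finds and caches the on-screen TutorialWidget.
; ProgressTutorial sets the first-person character's notebook flag, advances the tutorial, writes a discovery line to the NotebookWidget, then destroys the actor.
; GetString supplies its UI text, while IsInteractable returns false and WriteToNotebook returns empty text.
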(event EventBeginPlay
  (Utilities|FlowControl|Delay 0.1)
  (bind _foundwidgets (Widget|GetAllWidgetsOfClass "/Game/tutorialWidget.tutorialWidget_C" true))
  (for _array_element _foundwidgets
    (Variables|Default|SettutorialWidget _array_element)))

(event Collision|EventActorBeginOverlap
  (params (OtherActor :type Actor%20Object%20Reference)))

(event EventTick
  (params (DeltaSeconds :type Float%20%28single-precision%29)))

(fn ConstructionScript)

(fn ProgressTutorial
  (bind _asfirst_person_character (Utilities|Casting|CastToFirstPersonCharacter (Game|GetPlayerCharacter 0)))
  (Default|SetHasNotebook _asfirst_person_character true)
  (Default|GotoNextStage (Variables|Default|GettutorialWidget))
  (bind _foundwidgets (Widget|GetAllWidgetsOfClass "/Game/NotebookWidget.NotebookWidget_C" true))
  (Default|AddText (Utilities|Array|Get(acopy) _foundwidgets) "I found this note book.")
  (Actor|DestroyActor))

(fn GetString
  (return (Variables|Default|GetuiText)))

(fn IsInteractable
  (return false))

(fn WritetoNotebook
  (return ""))