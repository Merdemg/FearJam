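; CameraBP is a Blueprint that exposes a UI label and interaction queries, reporting itself as non-interactable with no notebook text.
; On BeginPlay it waits briefly, then searches top-level widgets for the TutorialWidget and stores a reference, which no other graph here uses.
; GetString returns its UiText variable as a Name, while IsInteractable and WriteToNotebook return fixed false and empty values.
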(event EventBeginPlay
  (Utilities|FlowControl|Delay 0.1)
  (bind _foundwidgets (Widget|GetAllWidgetsOfClass "/Game/tutorialWidget.tutorialWidget_C" true))
  (for _array_element _foundwidgets
    (Variables|Default|SettutorialWidget _array_element)))

(event Collision|EventActorBeginOverlap
  (params (OtherActor :type Actor%20Object%20Reference)))

(event EventTick
  (params (DeltaSeconds :type Float%20%28single-precision%29)))

(fn ConstructionScript)

(fn GetString
  (return (Utilities|String|StringToName (Variables|Default|GetuiText))))

(fn IsInteractable
  (return false))

(fn WritetoNotebook
  (return ""))