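; Heart Blueprint is an interactable heart that gets stabbed with knives and loads a level once it has taken enough.
; GetStabbed shows the Knife component, increments a knife counter and opens LevelToLoad when the count equals NumKnivesRequired.
; GetString returns the UiText value, and the construction script is empty.
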(fn ConstructionScript)

(fn GetStabbed
  (Rendering|SetVisibility (Variables|Default|GetKnife) true false)
  (Development|PrintString "got stabbed!!!")
  (bind _result (Math|Integer|IncrementInt (Variables|Default|GetnumOfKnives))
    (:%20%20
      (Variables|Default|SetnumOfKnives _result)
      (Math|Integer|CompareInt (Variables|Default|GetnumOfKnives) (Variables|Default|GetnumKnivesRequired)
        (:==
          (Game|OpenLevel(byName) (Variables|Default|GetlevelToLoad)))))))

(fn GetString
  (return (Variables|Default|GetuiText)))